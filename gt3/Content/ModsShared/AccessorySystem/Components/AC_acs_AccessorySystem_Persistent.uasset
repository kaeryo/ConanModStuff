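; Persistent variant of the accessory system component, letting players manage accessories and artisan armour looks on characters, owned thralls and placeables.
; On the locally controlled character, it injects wardrobe entry points into the inventory paperdoll and radial menu, with ownership or PvP loot checks.
; RPCs edit the target component's accessory list, whose OnRep reruns system init, and multicast armour and dye layout changes.
; Third-person camera toggles refresh accessory visuals.
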(event Custom|RadialMenuActivated
  (params (module :type GUI%20Module%20Object%20Reference) (isActive :type Boolean))
  (bind _returnvalue (|GetServerSettings))
  (bind _windowroot (|GUIModuleActivate module isActive false false)
    (:OnActivate
      (bind _asfun_combat_player_controller (Utilities|Casting|CastToFunCombat_PlayerController (Game|GetPlayerController 0)))
      (bind _aspersistent_humanoid_npc (Utilities|Casting|CastToPersistentHumanoidNPC (Utilities|ToObject(Interface) (Variables|/Game/Systems/InteractionManager.InteractionManager_C|GetSelectedObject (Default|GetInteractionManager _asfun_combat_player_controller))))
        (:then
          (if (CallFunction|HasOwnership _aspersistent_humanoid_npc (Game|GetPlayerCharacter 0))
            (bind _asw_main_radial_menu (Utilities|Casting|CastToW_MainRadialMenu _windowroot :!label _label))
            (Utilities|IsValid (Variables|/Game/UI/RadialMenus/W_MainRadialMenu.W_MainRadialMenu_C|GetMenu _asw_main_radial_menu)
              (:Is%20Valid
                (bind _returnvalue_2 (Class|RadialMenu|AddItem (Variables|/Game/UI/RadialMenus/W_MainRadialMenu.W_MainRadialMenu_C|GetMenu _asw_main_radial_menu) "Manage Accessories" "" "/Game/UI/Textures/GUIs/MainRadialMenu/T_MainRadialMenuIconLootAll.T_MainRadialMenuIconLootAll" "None" -1))
                (EventDispatchers|BindEventtoSignalClicked _returnvalue_2 (delegate Custom|EventRadialMenuClick))))))
        (:CastFailed
          (bind _asbp_master_placeables (Utilities|Casting|CastToBP_Master_Placeables (Utilities|ToObject(Interface) (Variables|/Game/Systems/InteractionManager.InteractionManager_C|GetSelectedObject (Default|GetInteractionManager _asfun_combat_player_controller))))
            (:then
              (bind _canaccess (CallFunction|CanAccessPlaceable _asbp_master_placeables))
              (if _canaccess
                (goto _label)))
            (:CastFailed
              (bind _asbase_player_char (Utilities|Casting|CastToBasePlayerChar (Utilities|ToObject(Interface) (Variables|/Game/Systems/InteractionManager.InteractionManager_C|GetSelectedObject (Default|GetInteractionManager _asfun_combat_player_controller)))))
              (if (Math|Boolean|ANDBoolean (Class|ConanCharacter|InState _asbase_player_char "Unconscious") (Class|ServerSettings|GetPVPEnabled _returnvalue) (Class|ServerSettings|GetEverybodyCanLootCorpse _returnvalue))
                (goto _label)))))))))

(event Custom|CustomEvent
  ;[1 1 1] Add Accessory button to UI
  (CallFunction|OpenAccessoryUI (Variables|/Game/UI/Inventory/W_PaperdollPanel.W_PaperdollPanel_C|GetInspectedCharacter (stale Custom|InventoryActivated _asw_paperdoll_panel_2))))

(event Custom|InventoryActivated
  (params (module :type GUI%20Module%20Object%20Reference) (isActive :type Boolean))
  ;[1 1 1] Add Accessory button to UI
  (bind _windowroot (|GUIModuleActivate module isActive false false)
    (:OnActivate
      (Utilities|FlowControl|Delay 0.2)
      (bind _ascrafting_gui (Utilities|Casting|CastToCraftingGUI _windowroot))
      (bind _assize_box (Utilities|Casting|CastToSizeBox (Class|PanelWidget|GetChildat (Widget|GetParent (Widget|GetParent (Variables|/Game/UI/Inventory/CraftingGUI.CraftingGUI_C|GetInventoryView _ascrafting_gui))) 2)))
      (bind _asoverlay (Utilities|Casting|CastToOverlay (Class|PanelWidget|GetChildat _assize_box)))
      (bind _asw_paperdoll_panel (Utilities|Casting|CastToW_PaperdollPanel (Class|PanelWidget|GetChildat _asoverlay))
        (:then
          (bind _asoverlay_2 (Utilities|Casting|CastToOverlay (Widget|GetParent (Widget|GetParent (Variables|/Game/UI/Inventory/W_PaperdollPanel.W_PaperdollPanel_C|GetUICharacterDisplay _asw_paperdoll_panel)))))
          (bind _returnvalue (UserInterface|CreateWidget "/Game/ModsShared/AccessorySystem/UI/Framework/W_acs_InventoryButton.W_acs_InventoryButton_C" (Widget|GetOwningPlayer _asoverlay_2)))
          (Widget|Panel|AddChild _asoverlay_2 _returnvalue)
          (Layout|BorderSlot|SetPadding _returnvalue (Utilities|Struct|MakeMargin 15.0 5.7e+02 0.0 0.0) :!class /Script/UMG.UserWidget)
          (EventDispatchers|BindEventtoSignalInventoryButtonPressed _returnvalue (delegate Custom|CustomEvent_2)))
        (:CastFailed
          (bind _assize_box_2 (Utilities|Casting|CastToSizeBox (Class|PanelWidget|GetChildat (Widget|GetParent (Widget|GetParent (Variables|/Game/UI/Inventory/CraftingGUI.CraftingGUI_C|GetInventoryView _ascrafting_gui))) 4)))
          (bind _asoverlay_3 (Utilities|Casting|CastToOverlay (Class|PanelWidget|GetChildat _assize_box_2)))
          (bind _asw_paperdoll_panel_2 (Utilities|Casting|CastToW_PaperdollPanel (Class|PanelWidget|GetChildat _asoverlay_3)))
          (bind _asoverlay_4 (Utilities|Casting|CastToOverlay (Widget|GetParent (Widget|GetParent (Variables|/Game/UI/Inventory/W_PaperdollPanel.W_PaperdollPanel_C|GetUICharacterDisplay _asw_paperdoll_panel_2)))))
          (bind _returnvalue_2 (UserInterface|CreateWidget "/Game/ModsShared/AccessorySystem/UI/Framework/W_acs_InventoryButton.W_acs_InventoryButton_C" (Widget|GetOwningPlayer _asoverlay_4)))
          (Widget|Panel|AddChild _asoverlay_4 _returnvalue_2)
          (Layout|BorderSlot|SetPadding _returnvalue_2 (Utilities|Struct|MakeMargin 15.0 5.7e+02 0.0 0.0) :!class /Script/UMG.UserWidget)
          (EventDispatchers|BindEventtoSignalInventoryButtonPressed _returnvalue_2 (delegate Custom|CustomEvent)))))))

(event Custom|EventRadialMenuClick
  (params (menuEntry :type Radial%20Menu%20Entry%20Object%20Reference))
  (CallFunction|OpenAccessoryUI (Utilities|ToObject(Interface) (Variables|/Game/Systems/InteractionManager.InteractionManager_C|GetSelectedObject (Default|GetInteractionManager (stale Custom|RadialMenuActivated _asfun_combat_player_controller))))))

(event Custom|OnCharacterPossessedOnClient_Event_0
  (params (NewController :type Controller%20Object%20Reference) (Character :type Conan%20Character%20Object%20Reference))
  (bind _returnvalue (Class|GUIModuleController|GetGUIModuleController))
  ;[1 1 1] Listen for UI events
  (bind _returnvalue_2 (Class|GUIModuleController|GetModule _returnvalue "MainRadialMenu"))
  (EventDispatchers|BindEventtoSignalActivated _returnvalue_2 (EventDispatchers|CreateEvent :!event Custom|RadialMenuActivated))
  (bind _returnvalue_3 (Class|GUIModuleController|GetModule _returnvalue "CharacterInventory"))
  (EventDispatchers|BindEventtoSignalActivated _returnvalue_3 (EventDispatchers|CreateEvent :!event Custom|InventoryActivated))
  (bind _returnvalue_4 (Class|GUIModuleController|GetModule _returnvalue "CraftingGUI"))
  (EventDispatchers|BindEventtoSignalActivated _returnvalue_4 (EventDispatchers|CreateEvent :!event Custom|InventoryActivated))
  (bind _asbase_player_char (Utilities|Casting|CastToBasePlayerChar (Components|GetOwner)))
  (Components|Activation|BindEventtoOnComponentActivated (Variables|/Game/Characters/BasePlayerChar.BasePlayerChar_C|GetAdjustableCamera _asbase_player_char) (delegate Custom|ThirdPersonEnabled))
  (EventDispatchers|BindEventtoOnComponentDeactivated (Variables|/Game/Characters/BasePlayerChar.BasePlayerChar_C|GetAdjustableCamera _asbase_player_char) (delegate Custom|ThirdPersonDisabled)))

(event Custom|ThirdPersonEnabled
  (params (Component :type Actor%20Component%20Object%20Reference) (bReset :type Boolean))
  (CallFunction|UpdateAccessoryVisuals))

(event Custom|OpenAccessoryUI
  (params (InputPin :type Object%20Object%20Reference))
  (bind _returnvalue (Class|GUIModuleController|GetGUIModuleController))
  (bind _returnvalue_2 (Class|GUIModuleController|GetModule (Class|GUIModuleController|GetGUIModuleController) "acs_WardrobeGUI"))
  (if (Class|GUIModule|IsActive _returnvalue_2)
    (Class|GUIModuleController|ActivateModule _returnvalue "acs_WardrobeGUI" false false)
    (else
      (bind _returnvalue_3 (Class|GUIModuleController|ActivateModule _returnvalue "acs_WardrobeGUI" true false))
      (bind _asw_acs_wardrobe (Utilities|Casting|CastToW_acs_Wardrobe _returnvalue_3))
      (bind _asactor (Utilities|Casting|CastToActor InputPin))
      (Default|SetupWardrobeUI _asw_acs_wardrobe _asactor)
      (CallFunction|RPCSetInteractingActor _asactor))))

(event Custom|ThirdPersonDisabled
  (params (Component :type Actor%20Component%20Object%20Reference))
  (CallFunction|UpdateAccessoryVisuals))

(event Custom|CustomEvent_2
  ;[1 1 1] Add Accessory button to UI
  (CallFunction|OpenAccessoryUI (Variables|/Game/UI/Inventory/W_PaperdollPanel.W_PaperdollPanel_C|GetInspectedCharacter (stale Custom|InventoryActivated _asw_paperdoll_panel))))

(event EventBeginPlay
  (bind _returnvalue (Class|GUIModuleController|GetGUIModuleController))
  (|CallParentFunction)
  (bind _asconan_character (Utilities|Casting|CastToConanCharacter (Components|GetOwner)))
  (if (Pawn|IsLocallyControlled _asconan_character)
    ;[1 1 1] Listen for UI events
    (bind _returnvalue_2 (Class|GUIModuleController|GetModule _returnvalue "MainRadialMenu"))
    (EventDispatchers|BindEventtoSignalActivated _returnvalue_2 (EventDispatchers|CreateEvent :!event Custom|RadialMenuActivated))
    (bind _returnvalue_3 (Class|GUIModuleController|GetModule _returnvalue "CharacterInventory"))
    (EventDispatchers|BindEventtoSignalActivated _returnvalue_3 (EventDispatchers|CreateEvent :!event Custom|InventoryActivated))
    (bind _returnvalue_4 (Class|GUIModuleController|GetModule _returnvalue "CraftingGUI"))
    (EventDispatchers|BindEventtoSignalActivated _returnvalue_4 (EventDispatchers|CreateEvent :!event Custom|InventoryActivated))
    (bind _asbase_player_char (Utilities|Casting|CastToBasePlayerChar (Components|GetOwner)))
    (Components|Activation|BindEventtoOnComponentActivated (Variables|/Game/Characters/BasePlayerChar.BasePlayerChar_C|GetAdjustableCamera _asbase_player_char) (delegate Custom|ThirdPersonEnabled))
    (EventDispatchers|BindEventtoOnComponentDeactivated (Variables|/Game/Characters/BasePlayerChar.BasePlayerChar_C|GetAdjustableCamera _asbase_player_char) (delegate Custom|ThirdPersonDisabled))
    (else
      (EventDispatchers|AssignOnCharacterPossessedonClient _asconan_character (delegate Custom|OnCharacterPossessedOnClient_Event_0)))))

(event Custom|RPC_AddPersistentAccessory
  (params (TargetActor :type Actor%20Object%20Reference) (AccessoryInfo :type ST%20Accessory%20Info%20Structure))
  (bind _returnvalue (Actor|GetComponentbyClass TargetActor "AC_acs_AccessorySystem_Persistent_C"))
  (bind _persistentaccessorylist (Variables|AC_acs_AccessorySystem_Persistent_C|GetPersistentAccessoryList _returnvalue))
  (bind (_array_element _array_index) (Utilities|Array|ForEachLoopwithBreak _persistentaccessorylist :!label _label)
    (:LoopBody
      (if (== (.EquipLocation (Utilities|Struct|BreakST_AccessoryInfo _array_element)) (.EquipLocation (Utilities|Struct|BreakST_AccessoryInfo AccessoryInfo)))
        (Utilities|Array|RemoveIndex _persistentaccessorylist _array_index)
        (goto _label Break)))
    (:Completed
      (Utilities|Array|Add _persistentaccessorylist AccessoryInfo))))

(event Custom|RPC_SetInteractingActor
  (params (actor :type Actor%20Object%20Reference))
  (Class|ConanCharacter|SetInteractingActor (.AsConan%20Character (Utilities|Casting|CastToConanCharacter (Components|GetOwner))) actor ""))

(event Custom|RPC_RemovePersistentAccessory
  (params (Actor :type Actor%20Object%20Reference) (TemplateID :type Integer))
  (bind _returnvalue (Actor|GetComponentbyClass Actor "AC_acs_AccessorySystem_Persistent_C"))
  (for (_array_element _array_index) (Variables|AC_acs_AccessorySystem_Persistent_C|GetPersistentAccessoryList _returnvalue)
    (if (== (.TemplateID (Utilities|Struct|BreakST_AccessoryInfo _array_element)) TemplateID)
      (Utilities|Array|RemoveIndex (Variables|AC_acs_AccessorySystem_Persistent_C|GetPersistentAccessoryList _returnvalue) _array_index))))

(event Custom|Multicast_AddArtisanArmour
  (params (Layout :type Character%20Layout%20Structure))
  (Class|CharacterCustomizationComponent|SetCharacterLayout (Variables|Default|GetCustomisationComp) Layout true false))

(event Custom|RPC_AddArtisanArmour
  (params (Actor :type Actor%20Object%20Reference) (Slot :type CharacterBodySlots%20Enum) (ItemInfo :type ST%20Accessory%20Info%20Structure))
  (bind _asbp_pl_crafting_station (Utilities|Casting|CastToBP_PL_Crafting_Station Actor)
    (:then
      (bind _returnvalue (Default|GetArtisanThrallInventory _asbp_pl_crafting_station))
      (bind _asthrall_item (Utilities|Casting|CastToThrallItem (Class|ItemInventory|GetFirstItemAvailable _returnvalue)))
      (bind _outlayout (CallFunction|ApplyArtisanArmour (Variables|/Script/ConanSandbox.ThrallItem|GetThrallCharLayout _asthrall_item) Slot ItemInfo))
      (bind _structout (Utilities|Struct|SetmembersinCharacterLayout (Variables|/Script/ConanSandbox.ThrallItem|GetThrallCharLayout _asthrall_item) (.MeshLayout (Utilities|Struct|BreakCharacterLayout _outlayout)) (.ArmourDyeParams (Utilities|Struct|BreakCharacterLayout _outlayout))))
      (CallFunction|MulticastAddArtisanArmour (Actor|GetComponentbyClass Actor "AC_acs_AccessorySystem_Persistent_C") _structout))
    (:CastFailed
      (if (Utilities|DoesObjectImplementInterface Actor "/Script/ConanSandbox.HasCharacterLayoutInterface")
        (bind _layout (Class|HasCharacterLayoutInterface|GetCharacterLayout(Message) Actor))
        (bind _outlayout_2 (CallFunction|ApplyArtisanArmour _layout Slot ItemInfo))
        (bind _structout_2 (Utilities|Struct|SetmembersinCharacterLayout _layout (.MeshLayout (Utilities|Struct|BreakCharacterLayout _outlayout_2)) (.ArmourDyeParams (Utilities|Struct|BreakCharacterLayout _outlayout_2))))
        (Class|HasCharacterLayoutInterface|SetCharacterLayout(Message) Actor _structout_2 false)
        (CallFunction|MulticastAddArtisanArmour (Actor|GetComponentbyClass Actor "AC_acs_AccessorySystem_Persistent_C") _structout_2)))))

(fn GetVisualAccessories
  (return (Variables|Default|GetPersistentAccessoryList)))

(fn OnRepPersistentAccessoryList
  (CallFunction|SystemInit))

(fn OnRepArtisanArmourUpdated)

(fn ApplyArtisanArmour
  (params (Layout :type Character%20Layout%20Structure) (Slot :type CharacterBodySlots%20Enum) (ItemInfo :type ST%20Accessory%20Info%20Structure))
  (bind (_templateid _dyes) (Utilities|Struct|BreakST_AccessoryInfo ItemInfo))
  (Class|CharacterFunctionLibrary|SetCharacterMeshSlot (.MeshLayout (Utilities|Struct|BreakCharacterLayout Layout)) Slot _templateid)
  (CallFunction|ApplyDyes Layout Slot _dyes)
  (return Layout))

(fn ApplyDyes
  (params (Layout :type Character%20Layout%20Structure%20%28by%20ref%29) (Slot :type CharacterBodySlots%20Enum) (DyeParams :type Armour%20Slot%20Dye%20Params%20Structure%20%28by%20ref%29))
  (bind _armourdyeparams (Utilities|Struct|BreakCharacterLayout Layout))
  (switch Utilities|FlowControl|Switch|SwitchonCharacterBodySlots Slot
    (:Helmet
      (Utilities|Struct|SetmembersinCharacterArmourDyeParams _armourdyeparams DyeParams))
    (:Forearms
      (Utilities|Struct|SetmembersinCharacterArmourDyeParams _armourdyeparams DyeParams))
    (:Hands
      (Utilities|Struct|SetmembersinCharacterArmourDyeParams _armourdyeparams DyeParams))
    (:Upperbody
      (Utilities|Struct|SetmembersinCharacterArmourDyeParams _armourdyeparams DyeParams))
    (:Lowerbody
      (Utilities|Struct|SetmembersinCharacterArmourDyeParams _armourdyeparams DyeParams))
    (:Legs
      (Utilities|Struct|SetmembersinCharacterArmourDyeParams _armourdyeparams DyeParams))
    (:Feet
      (Utilities|Struct|SetmembersinCharacterArmourDyeParams _armourdyeparams DyeParams))))

(fn CanAccessPlaceable
  (params (Placeable :type BP%20Master%20Placeables%20Object%20Reference))
  (bind _returnvalue (Actor|GetComponentbyClass Placeable "/Game/Characters/BP_CharacterCustomizationComponent.BP_CharacterCustomizationComponent_C"))
  (Utilities|IsValid (Actor|GetComponentbyClass Placeable "AC_acs_AccessorySystem_Persistent_C")
    (:Is%20Valid
      (bind _asbp_pl_crafting_station (Utilities|Casting|CastToBP_PL_Crafting_Station Placeable)
        (:then
          (Utilities|IsValid (Variables|/Game/Systems/Building/Placeables/BP_PL_Crafting_Station.BP_PL_Crafting_Station_C|GetCurrentArtisanThrallItem _asbp_pl_crafting_station)
            (:Is%20Valid
              (if (Class|BuildableBase|IsOwner Placeable (Game|GetPlayerCharacter 0) false) :!label _label
                (return true)
                (else
                  _)))
            (:Is%20Not%20Valid
              (return false))))
        (:CastFailed
          (if (Components|Activation|IsActive _returnvalue)
            (if (Variables|/Script/ConanSandbox.CharacterCustomizationComponent|GetEnabled _returnvalue)
              (goto _label)
              (else
                _))))))
    (:Is%20Not%20Valid
      _))
  (return false))

(fn ResetAccessoryList
  (Variables|Default|SetAccessoryList (Variables|Default|GetPersistentAccessoryList))
  (return false))