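; Base-style placeable item container for the building system, which shows the ContainerInfo UI module when interacted with.
; On BeginPlay it sizes its inventory from the item table row of its source item template.
; If a journey event is configured, storing an item reports it to the last activating player's Exiles Journey component.
; The UseFluidPress event also fires a Siptah-specific variant.
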(event Custom|SignalItemAdded_Event_0
  (params (index :type Integer) (item :type Game%20Item%20Object%20Reference) (srcInventory :type Item%20Inventory%20Object%20Reference) (srcIndex :type Integer))
  (bind _interactinginstigator (Variables|Default|GetInteractingInstigator))
  (bind _journeyeventtriggeronstoringitem (Variables|Default|GetJourneyEventTriggerOnStoringItem))
  (bind _returnvalue (Pawn|GetControlledPawn _interactinginstigator))
  (bind _returnvalue_2 (Actor|GetComponentbyClass _returnvalue "/Game/Systems/Progression/BP_AC_ExilesJourney.BP_AC_ExilesJourney_C"))
  (bind _returnvalue_3 (Transformation|GetActorLocation _returnvalue))
  (Utilities|IsValid _interactinginstigator
    (:Is%20Valid
      (Utilities|IsValid _returnvalue_2
        (:Is%20Valid
          (Class|ExilesJourneyComponent|AddJourneyEvent _returnvalue_2 _journeyeventtriggeronstoringitem _returnvalue_3)
          (if (Utilities|Name|Equal(Name) _journeyeventtriggeronstoringitem "UseFluidPress")
            (Class|ExilesJourneyComponent|AddJourneyEvent _returnvalue_2 "Siptah_UseFluidPress" _returnvalue_3)))))))

(event EventInteractableActivate
  (params (Component :type Primitive%20Component%20Object%20Reference) (Instigator :type Player%20Controller%20Object%20Reference) (HitIndex :type Integer) (TriggeredFromRadialWheel :type Boolean))
  (|CallParentFunction Component Instigator HitIndex false)
  (Variables|Default|SetInteractingInstigator Instigator))

(event EventBeginPlay
  (|CallParentFunction)
  (bind _returnvalue (Utilities|GetDataTableRow "/Game/Items/ItemTable.ItemTable" (Utilities|String|StringToName (Utilities|String|ToString(Integer) (Variables|Default|GetSourceItemTemplateID))))
    (:then
      (Class|ItemInventory|SetMaxItemCount (Variables|Default|GetPlaceableInventory) (.ItemContainerSize (Utilities|Struct|BreakItemTableRow _returnvalue)))
      (if (Utilities|Name|NotEqual(Name) (Variables|Default|GetJourneyEventTriggerOnStoringItem) "None")
        (EventDispatchers|AssignSignalItemAdded (Variables|Default|GetPlaceableInventory) (delegate Custom|SignalItemAdded_Event_0))))))

(event EventActorBeginOverlap
  (params (OtherActor :type Actor%20Object%20Reference)))

(event EventTick
  (params (DeltaSeconds :type Float%20%28single-precision%29)))

(fn ConstructionScript
  (|CallParentFunction))

(fn InteractableGetUIModuleName
  (return "ContainerInfo"))