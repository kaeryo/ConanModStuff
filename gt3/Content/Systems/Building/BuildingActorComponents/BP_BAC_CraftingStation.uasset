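; Building actor component that makes a placed building an interactable crafting station with a crafting UI.
; On BeginPlay it loads and applies saved inventory through the owner's persistence components.
; Activation toggles CraftingGUI per player via the interacting actor, tracking open users in InteractingPlayers; cancelled interaction closes it.
; When the CraftingQueue's artisan slot receives a valid thrall, all interacting players get progress on the exceptional-crafting achievement.
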(event Custom|GiveAchievement
  (params (thrallItem :type Thrall%20Item%20Object%20Reference))
  (if (Utilities|IsValid thrallItem)
    (for _array_element (Variables|Default|GetInteractingPlayers)
      (Utilities|IsValid _array_element
        (:Is%20Valid
          (Utilities|IsValid (Pawn|GetController (.AsPawn (Utilities|Casting|CastToPawn _array_element)))
            (:Is%20Valid
              (bind _asachievement_interface (Utilities|Casting|CastToAchievementInterface (Class|Actor|GetComponentbyInterface (Pawn|GetController (.AsPawn (Utilities|Casting|CastToPawn _array_element))) "/Game/Systems/Achievements/AchievementInterface.AchievementInterface_C")))
              (Default|GiveAchievementProgressInterfaceFunc _asachievement_interface "ACH_CraftExceptional" 1e+02))))))))

(event EventInteractableActivate
  (params (Component :type Primitive%20Component%20Object%20Reference) (Instigator :type Player%20Controller%20Object%20Reference) (HitIndex :type Integer) (TriggeredFromRadialWheel :type Boolean))
  (bind _returnvalue (Pawn|GetControlledPawn Instigator))
  (if (Utilities|Array|ContainsItem (Variables|Default|GetInteractingPlayers) _returnvalue)
    (CallFunction|CloseUI _returnvalue)
    (else
      (bind _asconan_character (Utilities|Casting|CastToConanCharacter _returnvalue))
      (if (Class|ConanCharacter|IsPlayer _asconan_character)
        (Class|ConanCharacter|SetInteractingActor _asconan_character (Components|GetOwner) "CraftingGUI")
        (Utilities|Array|Add (Variables|Default|GetInteractingPlayers) _asconan_character)))))

(event EventBeginPlay
  (bind _returnvalue (Components|GetOwner))
  (|CallParentFunction)
  (for _array_element (Actor|GetComponentsByClass _returnvalue "/Script/ConanSandbox.ConanBuildingPersistenceComponent")
    (bind _result (|LoadInventory (Class|PersistenceComponent|GetUniqueID _array_element))
      (:OnSuccess
        (Class|LoadInventoryCallProxy|ProcessInventoryData (Components|GetOwner) _result))))
  (EventDispatchers|BindEventtoSignalArtisanSlotChanged (Actor|GetComponentbyClass _returnvalue "/Script/ConanSandbox.CraftingQueue") (delegate Custom|GiveAchievement)))

(event EventInteractableSelectionChanged
  (params (IsSelected :type Boolean) (Instigator :type Player%20Controller%20Object%20Reference) (InstanceIndex :type Integer))
  (bind _returnvalue (Pawn|GetControlledPawn Instigator))
  (if (and (not IsSelected) (Utilities|Array|ContainsItem (Variables|Default|GetInteractingPlayers) _returnvalue))
    (CallFunction|CloseUI _returnvalue)))

(event EventEndPlay
  (params (EndPlayReason :type EEndPlayReason%20Enum :default "Destroyed"))
  (|CallParentFunction EndPlayReason)
  (EventDispatchers|UnbindEventfromSignalArtisanSlotChanged (Actor|GetComponentbyClass (Components|GetOwner) "/Script/ConanSandbox.CraftingQueue") (delegate Custom|GiveAchievement)) ; Is this really needed?
)

(fn IsOpen
  (return (> (Utilities|Array|Length (Variables|Default|GetInteractingPlayers)) 0)))

(fn CloseUI
  (params (Character :type Pawn%20Object%20Reference))
  (Utilities|Array|RemoveItem (Variables|Default|GetInteractingPlayers) Character)
  (bind _asconan_character (Utilities|Casting|CastToConanCharacter Character))
  (bind _returnvalue (Class|ConanCharacter|GetInteractingActor _asconan_character))
  (if (== _returnvalue (Components|GetOwner))
    (Class|ConanCharacter|SetInteractingActor _asconan_character 0 "None")))