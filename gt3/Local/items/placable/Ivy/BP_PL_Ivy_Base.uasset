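; Base Blueprint for placeable ivy whose owner can pick one of four leaf or clover variants from the radial menu.
; Menu clicks send the variant ID through an RPC on the player pawn's IvyComponent.
; ChangeMaterial stores the replicated MaterialId and marks building persistence dirty.
; BeginPlay and OnRep apply the matching data table material, keeping the mesh hidden if no row matches.
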(event Custom|Change%20Material
  (params (id%20reference :type Integer))
  (Variables|Default|SetmaterialId id%20reference)
  (Class|PersistenceComponent|SetDirty (Variables|Default|GetConanBuildingPersistence) true 5.0))

(event Custom|Variant%20IV
  (params (menuEntry :type Radial%20Menu%20Entry%20Object%20Reference))
  (Default|RPCChangeIvyMaterial (Actor|GetComponentbyClass (Pawn|GetControlledPawn (Widget|GetOwningPlayer (stale EventInteractableMenu RadialMenu))) "/Game/Mods/gt3/items/placable/Ivy/IvyComponent.IvyComponent_C") self 4))

(event Custom|Variant%20I
  (params (menuEntry :type Radial%20Menu%20Entry%20Object%20Reference))
  (Default|RPCChangeIvyMaterial (Actor|GetComponentbyClass (Pawn|GetControlledPawn (Widget|GetOwningPlayer (stale EventInteractableMenu RadialMenu))) "/Game/Mods/gt3/items/placable/Ivy/IvyComponent.IvyComponent_C") self 1))

(event Custom|Variant%20III
  (params (menuEntry :type Radial%20Menu%20Entry%20Object%20Reference))
  (Default|RPCChangeIvyMaterial (Actor|GetComponentbyClass (Pawn|GetControlledPawn (Widget|GetOwningPlayer (stale EventInteractableMenu RadialMenu))) "/Game/Mods/gt3/items/placable/Ivy/IvyComponent.IvyComponent_C") self 3))

(event Custom|FixMaterial
  (bind _staticmesh (Variables|Default|GetStaticMesh))
  (Rendering|SetVisibility _staticmesh false false)
  (bind _returnvalue (Utilities|GetDataTableRow "/Game/Mods/gt3/items/placable/Ivy/Ivy_Material_Table.Ivy_Material_Table" (Utilities|String|StringToName (Utilities|String|ToString(Integer) (Variables|Default|GetmaterialId))))
    (:then
      (Rendering|Material|SetMaterial _staticmesh 0 (Utilities|Struct|BreakIvy_Material_Reference _returnvalue))
      (Rendering|SetVisibility _staticmesh true false))))

(event Custom|Variant%20II
  (params (menuEntry :type Radial%20Menu%20Entry%20Object%20Reference))
  (Default|RPCChangeIvyMaterial (Actor|GetComponentbyClass (Pawn|GetControlledPawn (Widget|GetOwningPlayer (stale EventInteractableMenu RadialMenu))) "/Game/Mods/gt3/items/placable/Ivy/IvyComponent.IvyComponent_C") self 2))

(event EventBeginPlay
  (|CallParentFunction)
  (CallFunction|FixMaterial))

(event Collision|EventActorBeginOverlap
  (params (OtherActor :type Actor%20Object%20Reference)))

(event EventTick
  (params (DeltaSeconds :type Float%20%28single-precision%29)))

(event EventInteractableMenu
  (params (RadialMenu :type Radial%20Menu%20Object%20Reference) (HitIndex :type Integer))
  (|CallParentFunction RadialMenu HitIndex)
  (if (Class|BuildableBase|IsOwner (Pawn|GetControlledPawn (Widget|GetOwningPlayer RadialMenu)) false)
    (Utilities|IsValid RadialMenu
      (:Is%20Valid
        (bind _returnvalue (Class|RadialMenu|AddItem RadialMenu "Variants" "Change the look of your leaves" "/Game/Mods/gt3/items/placable/Ivy/Textures/Ivy_Small.Ivy_Small" "None" -1))
        (bind _returnvalue_2 (Class|RadialMenuEntry|AddSubItem _returnvalue "Variant I" "Green leaves" "/Game/Mods/gt3/items/placable/Ivy/Textures/T_VariantIcon1.T_VariantIcon1" "None" -1))
        (EventDispatchers|BindEventtoSignalClicked _returnvalue_2 (delegate Custom|Variant%20I))
        (bind _returnvalue_3 (Class|RadialMenuEntry|AddSubItem _returnvalue "Variant II" "Red leaves" "/Game/Mods/gt3/items/placable/Ivy/Textures/T_VariantIcon2.T_VariantIcon2" "None" -1))
        (EventDispatchers|BindEventtoSignalClicked _returnvalue_3 (delegate Custom|Variant%20II))
        (bind _returnvalue_4 (Class|RadialMenuEntry|AddSubItem _returnvalue "Variant III" "Green clovers" "/Game/Mods/gt3/items/placable/Ivy/Textures/T_VariantIcon3.T_VariantIcon3" "None" -1))
        (EventDispatchers|BindEventtoSignalClicked _returnvalue_4 (delegate Custom|Variant%20III))
        (bind _returnvalue_5 (Class|RadialMenuEntry|AddSubItem _returnvalue "Variant II" "Green/Yellow clovers" "/Game/Mods/gt3/items/placable/Ivy/Textures/T_VariantIcon4.T_VariantIcon4" "None" -1))
        (EventDispatchers|BindEventtoSignalClicked _returnvalue_5 (delegate Custom|Variant%20IV))))))

(fn ConstructionScript)

(fn OnRepMaterialId
  (CallFunction|FixMaterial))